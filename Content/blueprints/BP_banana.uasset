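; BP_banana is a collectible banana pickup for the third-person character.
; On BeginPlay it scales its static mesh down, then spins it every Tick with a fixed local rotation that is not scaled by delta time.
; When a BP_ThirdPersonCharacter overlaps it, it increments the Fruits count on BP_ThirdPersonGameMode and destroys itself.
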(event `self.ReceiveBeginPlay`
  (`SceneComponent.SetWorldScale3D` (`self.StaticMesh`) (0.09 0.09 0.09)))

(event `self.ReceiveActorBeginOverlap`
  (params (OtherActor :type "Actor Object Reference"))
  (cast `/Game/ThirdPerson/Blueprints/BP_ThirdPersonCharacter` OtherActor)
  (bind _asbp_third_person_game_mode (cast `/Game/ThirdPerson/Blueprints/BP_ThirdPersonGameMode` (`GameplayStatics.GetGameMode`)))
  (set `/Game/ThirdPerson/Blueprints/BP_ThirdPersonGameMode.fruits` (+ (`/Game/ThirdPerson/Blueprints/BP_ThirdPersonGameMode.fruits` _asbp_third_person_game_mode) 1) _asbp_third_person_game_mode)
  (`self.K2_DestroyActor`))

(event `self.ReceiveTick`
  (params (DeltaSeconds :type "Float (single-precision)"))
  (`SceneComponent.K2_AddLocalRotation` (`self.StaticMesh`) (`KismetMathLibrary.MakeRotator` 1.0 0.0 2.0) false false))

(fn `UserConstructionScript`)